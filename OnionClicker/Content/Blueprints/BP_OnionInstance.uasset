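; Central instance for an idle onion game, holding onion count, onions per second (OPS), shop entries and save state.
; Init polls for the HUD, then fetches Amsterdam time through VaRest to load or create the save and credit offline earnings since its timestamp.
; A self-calling one-second delay loop adds OPS to onions and refreshes the HUD stats.
; BuyItem raises an entry's owned count and cost, then saves.
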(event Custom|SaveGame
  ;[0.4644 0.8795 1] Save Game
  (Variables|/Game/Blueprints/BP_OnionSaveGameObject.BP_OnionSaveGameObject_C|SetKitchenSaveStruct (Variables|Default|GetOnionSaveGameObjRef) (Utilities|Struct|MakeStruct_KitchenSave (Variables|Default|GetOPS) (Variables|Default|GetOnions) (Variables|Default|GetKitchenName) (Variables|Default|GetShopEntryStruct) (Variables|Default|GetTimeStructRef)))
  (SaveGame|SaveGametoSlot (Variables|Default|GetOnionSaveGameObjRef) "onion"))

(event Custom|InitializeSaves
  ;[1 1 1] Stats Save - Creates save if one is abscent.
  (bind _returnvalue (SaveGame|DoesSaveGameExist "onion"))
  (if _returnvalue
    (bind _returnvalue_2 (SaveGame|LoadGamefromSlot "onion"))
    (bind _asbp_onion_save_game_object (Utilities|Casting|CastToBP_OnionSaveGameObject _returnvalue_2))
    (bind _output_get (Variables|Default|SetOnionSaveGameObjRef _asbp_onion_save_game_object))
    (Variables|Default|SetOPS (.ops (Variables|/Game/Blueprints/BP_OnionSaveGameObject.BP_OnionSaveGameObject_C|GetKitchenSaveStruct _output_get)))
    (Variables|Default|SetOnions (.onions (Variables|/Game/Blueprints/BP_OnionSaveGameObject.BP_OnionSaveGameObject_C|GetKitchenSaveStruct _output_get)))
    (Variables|Default|SetKitchenName (.name (Variables|/Game/Blueprints/BP_OnionSaveGameObject.BP_OnionSaveGameObject_C|GetKitchenSaveStruct _output_get)))
    (Variables|Default|SetShopEntryStruct (.storeentries (Variables|/Game/Blueprints/BP_OnionSaveGameObject.BP_OnionSaveGameObject_C|GetKitchenSaveStruct _output_get)))
    (Variables|Default|SetSavedTimeSpan (Math|Timespan|MakeTimespan (.Days (Utilities|Struct|BreakStruct_Time (.timestruct (Variables|/Game/Blueprints/BP_OnionSaveGameObject.BP_OnionSaveGameObject_C|GetKitchenSaveStruct _output_get)))) (.Hours (Utilities|Struct|BreakStruct_Time (.timestruct (Variables|/Game/Blueprints/BP_OnionSaveGameObject.BP_OnionSaveGameObject_C|GetKitchenSaveStruct _output_get)))) (.Minutes (Utilities|Struct|BreakStruct_Time (.timestruct (Variables|/Game/Blueprints/BP_OnionSaveGameObject.BP_OnionSaveGameObject_C|GetKitchenSaveStruct _output_get)))) (.Seconds (Utilities|Struct|BreakStruct_Time (.timestruct (Variables|/Game/Blueprints/BP_OnionSaveGameObject.BP_OnionSaveGameObject_C|GetKitchenSaveStruct _output_get))))))
    (CallFunction|GenerateOfflineRevenue (Math|Float|Round (- (Math|Timespan|GetTotalSeconds (Variables|Default|GetCurrentTimeSpan)) (Math|Timespan|GetTotalSeconds (Variables|Default|GetSavedTimeSpan)))))
    (Default|InitializeStats (Variables|Default|GetHudRef))
    (CallFunction|SaveGame)
    (else
      (bind _returnvalue_3 (SaveGame|CreateSaveGameObject "/Game/Blueprints/BP_OnionSaveGameObject.BP_OnionSaveGameObject_C"))
      (Variables|/Game/Blueprints/BP_OnionSaveGameObject.BP_OnionSaveGameObject_C|SetKitchenSaveStruct _returnvalue_3 (Utilities|Struct|MakeStruct_KitchenSave (Variables|Default|GetOPS) (Variables|Default|GetOnions) (Variables|Default|GetKitchenName) (Variables|Default|GetShopEntryStruct) (Variables|Default|GetTimeStructRef)))
      (SaveGame|SaveGametoSlot _returnvalue_3 "onion")
      (CallFunction|InitializeSaves))))

(event Custom|TickInitialize
  ;[0.7715 1 0.5828] Initiate Timer then Tick over
  (Utilities|FlowControl|DoOnce false
    (:Completed
      (Utilities|FlowControl|Delay 2.0)
      (CallFunction|Tick))))

(event Custom|Tick
  ;[0.7715 1 0.5828] Initiate Timer then Tick over
  (Utilities|FlowControl|Delay 1.0)
  (Variables|Default|SetOnions (+ (Variables|Default|GetOnions) (Variables|Default|GetOPS)))
  (Default|Update (Variables|/Game/Interface/BP_HUD.BP_HUD_C|GetBP_StatsWidg (Variables|Default|GetHudRef)))
  (CallFunction|Tick))

(event Custom|GetTime
  (bind _returnvalue (|VaRestSubsystem))
  ;[0.4225 0.5105 1] VaRest - JSON Time Format
  (bind _returnvalue_2 (Class|VaRestSubsystem|ConstructVaRestJsonObject _returnvalue))
  (Class|VaRestSubsystem|CallURL _returnvalue "https://timeapi.io/api/Time/current/zone?timeZone=Europe%2FAmsterdam" "GET" "json" _returnvalue_2 (delegate Custom|TimeDate)))

(event Custom|TimeDate
  (params (Request :type Va%20Rest%20Request%20JSON%20Object%20Reference))
  (bind _returnvalue (Class|VaRestRequestJSON|GetResponseObject Request))
  ;[0.4225 0.5105 1] VaRest - JSON Time Format
  (for _index (range 0 5)
    (switch int _index
      (:0
        (Variables|Default|SetYears (Math|Conversions|ToInteger(Byte) (Class|VaRestJsonValue|AsInt64 (Class|VaRestJsonObject|GetField _returnvalue (Utilities|Array|Get(acopy) (Class|VaRestJsonObject|GetFieldNames _returnvalue) _index))))))
      (:1
        (Variables|Default|SetMonths (Math|Conversions|ToInteger(Byte) (Class|VaRestJsonValue|AsInt64 (Class|VaRestJsonObject|GetField _returnvalue (Utilities|Array|Get(acopy) (Class|VaRestJsonObject|GetFieldNames _returnvalue) _index))))))
      (:2
        (Variables|Default|SetDays (Math|Conversions|ToInteger(Byte) (Class|VaRestJsonValue|AsInt64 (Class|VaRestJsonObject|GetField _returnvalue (Utilities|Array|Get(acopy) (Class|VaRestJsonObject|GetFieldNames _returnvalue) _index))))))
      (:3
        (Variables|Default|SetHours (Math|Conversions|ToInteger(Byte) (Class|VaRestJsonValue|AsInt64 (Class|VaRestJsonObject|GetField _returnvalue (Utilities|Array|Get(acopy) (Class|VaRestJsonObject|GetFieldNames _returnvalue) _index))))))
      (:4
        (Variables|Default|SetMinutes (Math|Conversions|ToInteger(Byte) (Class|VaRestJsonValue|AsInt64 (Class|VaRestJsonObject|GetField _returnvalue (Utilities|Array|Get(acopy) (Class|VaRestJsonObject|GetFieldNames _returnvalue) _index))))))
      (:5
        (Variables|Default|SetSeconds (Math|Conversions|ToInteger(Byte) (Class|VaRestJsonValue|AsInt64 (Class|VaRestJsonObject|GetField _returnvalue (Utilities|Array|Get(acopy) (Class|VaRestJsonObject|GetFieldNames _returnvalue) _index))))))))
  (Variables|Default|SetTimeStructRef (Utilities|Struct|MakeStruct_Time (Variables|Default|GetSeconds) (Variables|Default|GetMinutes) (Variables|Default|GetHours) (Variables|Default|GetDays) (Variables|Default|GetMonths) (Variables|Default|GetYears)))
  (Variables|Default|SetCurrentTimeSpan (Class|KismetMathLibrary|MakeTimespan2 (Variables|Default|GetDays) (Variables|Default|GetHours) (Variables|Default|GetMinutes) (Variables|Default|GetSeconds)))
  (CallFunction|InitializeSaves))

(event EventInit
  ;[0.9173 0.4892 1] Initializes HUD after ready check.
  (Utilities|FlowControl|Sequence
    (:then_0
      (bind _foundwidgets (Widget|GetAllWidgetsOfClass "/Game/Interface/BP_HUD.BP_HUD_C" true :!label _label))
      (bind _output_get (Variables|Default|SetHudRef (Utilities|Array|Get(acopy) _foundwidgets)))
      (Utilities|IsValid _output_get
        (:Is%20Valid
          (CallFunction|GetTime))
        (:Is%20Not%20Valid
          (Utilities|FlowControl|Delay 0.01)
          (goto _label))))
    (:then_1
      (CallFunction|TickInitialize))))

(fn CalculateOPS
  (for _array_element (Variables|Default|GetShopEntryStruct)
    (LocalVariables|SetCurrentOPS (+ (LocalVariables|GetCurrentOPS) (* (.AmountOwned (Utilities|Struct|BreakStruct_ShopEntry _array_element)) (.OPS (Utilities|Struct|BreakStruct_ShopEntry _array_element))))))
  (LocalVariables|SetCurrentOPS (LocalVariables|GetCurrentOPS))
  (return))

(fn BuyItem
  (params (Item :type Struct%20Shop%20Entry%20Structure) (Quantity :type Integer))
  (bind _shopentrystruct (Variables|Default|GetShopEntryStruct))
  (LocalVariables|SetItemLocal Item)
  (LocalVariables|SetQuantityLocal Quantity)
  (Utilities|Array|SetArrayElem (Variables|Default|GetShopEntryStruct) (Utilities|Array|FindItem _shopentrystruct (LocalVariables|GetItemLocal)) (Utilities|Struct|MakeStruct_ShopEntry (.Name (Utilities|Struct|BreakStruct_ShopEntry (Utilities|Array|Get(acopy) _shopentrystruct (Utilities|Array|FindItem _shopentrystruct (LocalVariables|GetItemLocal))))) (.Icon (Utilities|Struct|BreakStruct_ShopEntry (Utilities|Array|Get(acopy) _shopentrystruct (Utilities|Array|FindItem _shopentrystruct (LocalVariables|GetItemLocal))))) (* (.Cost (Utilities|Struct|BreakStruct_ShopEntry (Utilities|Array|Get(acopy) _shopentrystruct (Utilities|Array|FindItem _shopentrystruct (LocalVariables|GetItemLocal))))) 1.4) true (+ (.AmountOwned (Utilities|Struct|BreakStruct_ShopEntry (Utilities|Array|Get(acopy) _shopentrystruct (Utilities|Array|FindItem _shopentrystruct (LocalVariables|GetItemLocal))))) (LocalVariables|GetQuantityLocal)) (.OPS (Utilities|Struct|BreakStruct_ShopEntry (Utilities|Array|Get(acopy) _shopentrystruct (Utilities|Array|FindItem _shopentrystruct (LocalVariables|GetItemLocal)))))) true)
  (CallFunction|SaveGame)
  (return))

(fn GenerateOfflineRevenue
  (params (Seconds :type Integer))
  (bind _ops (Variables|Default|GetOPS))
  (bind _returnvalue (* _ops Seconds))
  (Variables|Default|SetOnions (+ (Variables|Default|GetOnions) _returnvalue))
  (Development|PrintString (Utilities|String|Append "Offline for" (Utilities|String|ToString(Integer) Seconds) "Seconds. Generated" (Utilities|String|ToString(Float) _returnvalue) "Onions"))
  (return))